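; Base NPC Blueprint that runs voiced dialogue when the third-person character enters its collision sphere.
; Overlap registers the NPC on the player, shows a dialogue widget and calls NextLine.
; NextLine steps through DT_NPC_Dialogue rows from IndexStart, setting text and voice audio, and aligning text left for NPC or right for Player.
; An empty row, the table's end or leaving the sphere closes and resets the dialogue.
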(event OnComponentBeginOverlap(Sphere_Collision)
  (params (OverlappedComponent :type Primitive%20Component%20Object%20Reference) (OtherActor :type Actor%20Object%20Reference) (OtherComp :type Primitive%20Component%20Object%20Reference) (OtherBodyIndex :type Integer) (bFromSweep :type Boolean) (SweepResult :type Hit%20Result%20Structure%20%28by%20ref%29))
  ;[0.15 0.15 0.15 0.5] Spawn Dialogue Widget
  (bind _asbp_third_person_character (Utilities|Casting|CastToBP_ThirdPersonCharacter OtherActor))
  (bind _output_get (Variables|Default|SetPlayer _asbp_third_person_character))
  (Variables|/Game/ThirdPerson/Blueprints/BP_ThirdPersonCharacter.BP_ThirdPersonCharacter_C|SetBP_NPC _output_get self)
  (UserInterface|Viewport|AddtoViewport (Variables|Default|GetW_Dialogue) 0)
  (CallFunction|NextLine))

(event OnComponentEndOverlap(Sphere_Collision)
  (params (OverlappedComponent :type Primitive%20Component%20Object%20Reference) (OtherActor :type Actor%20Object%20Reference) (OtherComp :type Primitive%20Component%20Object%20Reference) (OtherBodyIndex :type Integer))
  ;[0.15 0.15 0.15 0.5] Hidden and Dead when leaving
  (Utilities|Casting|CastToBP_ThirdPersonCharacter OtherActor)
  (CallFunction|EndDialogue))

(event Custom|Next%20Line
  (bind _w_dialogue (Variables|Default|GetW_Dialogue))
  (bind _audio_component (Variables|Default|GetAudio_Component))
  (bind _fishermen_dialogue (Variables|/Game/Dev/Bps/Widgets/WBP_Dialogue.WBP_Dialogue_C|GetFishermen_Dialogue _w_dialogue))
  ;[0.15 0.15 0.15 0.5] New Dialogue System
  (bind _outrownames (DataTable|GetDataTableRowNames "/Game/Dev/Bps/NPC/DT_NPC_Dialogue.DT_NPC_Dialogue"))
  (if (> (Variables|Default|GetLine_Index) (Utilities|Array|LastIndex _outrownames))
    (CallFunction|EndDialogue)
    (else
      (bind _returnvalue (Utilities|GetDataTableRow "/Game/Dev/Bps/NPC/DT_NPC_Dialogue.DT_NPC_Dialogue" (Utilities|Array|Get(acopy) _outrownames (Variables|Default|GetLine_Index)))
        (:then
          (if (Utilities|Enum|Equal(Enum) (.dialogue _returnvalue) (Utilities|Text|MakeLiteralText "")) ; Are we at the end of this character's lines?
            (CallFunction|EndDialogue)
            (else
              (Rendering|Components|TextRender|SetText (Variables|/Game/Dev/Bps/Widgets/WBP_Dialogue.WBP_Dialogue_C|GetFishermen_Dialogue (Variables|Default|GetW_Dialogue)) (.dialogue _returnvalue))
              (Math|Integer|IncrementInt (Variables|Default|GetLine_Index)
                (:%20%20
                  (Audio|Components|Audio|SetSound _audio_component (.voiceddialogue _returnvalue))
                  (Audio|Components|Audio|Play _audio_component 0.0)
                  (switch Utilities|FlowControl|Switch|SwitchonE_Speaker (.speaker _returnvalue)
                    (:NewEnumerator0
                      (Class|Widget|SetRenderTransformAngle _fishermen_dialogue (Math|Random|RandomFloatinRange 0.0 0.0))
                      (Variables|/Script/UMG.TextLayoutWidget|SetJustification _fishermen_dialogue "Left"))
                    (:NewEnumerator1
                      (Class|Widget|SetRenderTransformAngle _fishermen_dialogue (Math|Random|RandomFloatinRange 0.0 0.0))
                      (Variables|/Script/UMG.TextLayoutWidget|SetJustification _fishermen_dialogue "Right"))))))))))))

(event Custom|End%20Dialogue
  ;[0.15 0.15 0.15 0.5] End Dialogue
  (Widget|RemovefromParent (Variables|Default|GetW_Dialogue)) ; Hide the widget
  (Variables|Default|SetLine_Index (Variables|Default|GetIndex%20Start)) ; Reset the Index
  (Variables|/Game/ThirdPerson/Blueprints/BP_ThirdPersonCharacter.BP_ThirdPersonCharacter_C|SetBP_NPC (Variables|Default|GetPlayer) 0) ; Tell the player to forget about us
  (Variables|Default|SetPlayer 0) ; Forget about the player
)

(event EventBeginPlay
  ;[0.15 0.15 0.15 0.5] Create Widget
  (bind _returnvalue (UserInterface|CreateWidget "/Game/Dev/Bps/Widgets/WBP_Dialogue.WBP_Dialogue_C"))
  (Variables|Default|SetW_Dialogue _returnvalue)
  (Variables|Default|SetLine_Index (Variables|Default|GetIndex%20Start)))

(fn ConstructionScript)