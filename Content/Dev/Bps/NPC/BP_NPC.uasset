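; NPC Blueprint that shows line-by-line dialogue when the third-person character enters its collision sphere.
; It creates a dialogue widget at BeginPlay, adds it to the viewport on overlap and registers itself on the player as BPNPC.
; NextLine writes the current Dialogue array entry to the widget and increments the index, which is never reset or bounds-checked here.
; Any end overlap removes all widgets from the viewport.
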(event OnComponentBeginOverlap(Sphere_Collision)
  (params (OverlappedComponent :type Primitive%20Component%20Object%20Reference) (OtherActor :type Actor%20Object%20Reference) (OtherComp :type Primitive%20Component%20Object%20Reference) (OtherBodyIndex :type Integer) (bFromSweep :type Boolean) (SweepResult :type Hit%20Result%20Structure%20%28by%20ref%29))
  ;[0.15 0.15 0.15 0.5] Spawn Dialogue Widget
  (bind _asbp_third_person_character (Utilities|Casting|CastToBP_ThirdPersonCharacter OtherActor))
  (bind _output_get (Variables|Default|SetPlayer _asbp_third_person_character))
  (Variables|/Game/ThirdPerson/Blueprints/BP_ThirdPersonCharacter.BP_ThirdPersonCharacter_C|SetBP_NPC _output_get self)
  (UserInterface|Viewport|AddtoViewport (Variables|Default|GetW_Dialogue) 0)
  (CallFunction|NextLine))

(event OnComponentEndOverlap(Sphere_Collision)
  (params (OverlappedComponent :type Primitive%20Component%20Object%20Reference) (OtherActor :type Actor%20Object%20Reference) (OtherComp :type Primitive%20Component%20Object%20Reference) (OtherBodyIndex :type Integer))
  ;[0.15 0.15 0.15 0.5] Comment
  (Viewport|RemoveAllWidgets))

(event Custom|Next%20Line
  ;[0.15 0.15 0.15 0.5] Next Line
  (Rendering|Components|TextRender|SetText (Variables|/Game/Dev/Bps/Widgets/WBP_Dialogue.WBP_Dialogue_C|GetFishermen_Dialogue (Variables|Default|GetW_Dialogue)) (Utilities|Array|Get(acopy) (Variables|Default|GetDialogue) (Variables|Default|GetLine_Index)))
  (Math|Integer|IncrementInt (Variables|Default|GetLine_Index)))

(event EventBeginPlay
  ;[0.15 0.15 0.15 0.5] Create Widget
  (bind _returnvalue (UserInterface|CreateWidget "/Game/Dev/Bps/Widgets/WBP_Dialogue.WBP_Dialogue_C"))
  (Variables|Default|SetW_Dialogue _returnvalue))

(fn ConstructionScript)